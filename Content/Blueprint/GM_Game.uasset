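; GM_Game is a game Blueprint that assigns toy orders to customers.
; On BeginPlay it caches every BP_Customer actor in the level and calls SpawnRandomOrder once.
; SpawnRandomOrder rebuilds the list of customers without an order, picks one at random, and starts an order on it using a random row name from the DTToys data table.
; It does nothing when no customer is free.
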(event EventBeginPlay
  (bind _outactors (Actor|GetAllActorsOfClass "/Game/Blueprint/Commandes/BP_Customer.BP_Customer_C"))
  (Variables|Default|SetAllCustomers _outactors)
  (CallFunction|SpawnRandomOrder))

(fn ConstructionScript)

(fn SpawnRandomOrder
  (bind _availablecustomers (LocalVariables|GetAvailableCustomers))
  (bind _returnvalue (Utilities|Array|Length _availablecustomers))
  (Utilities|Array|Clear (LocalVariables|GetAvailableCustomers))
  (for _array_element (Variables|Default|GetAllCustomers)
    (if (not (Variables|/Game/Blueprint/Commandes/BP_Customer.BP_Customer_C|GetHasOrder? _array_element))
      (Utilities|Array|Add (LocalVariables|GetAvailableCustomers) _array_element)))
  (if (> _returnvalue 0)
    (bind _output_get (LocalVariables|SetSelectedCustomer (Utilities|Array|Get(acopy) (LocalVariables|GetAvailableCustomers) (Math|Random|RandomInteger _returnvalue))))
    (bind _outrownames (DataTable|GetDataTableRowNames (Variables|Default|GetDT_Toys)))
    (Default|StartOrder _output_get (Utilities|Array|Get(acopy) _outrownames (Math|Random|RandomInteger (Utilities|Array|Length _outrownames))))
    (return)
    (else
      (return))))