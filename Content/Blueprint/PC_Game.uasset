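; PC_Game is the in-game player controller that sets up the player's pawn, camera and input for picking up and dropping objects.
; On BeginPlay it possesses the level's BP_Character, switches the view to a separate BP_CharacterCamera actor and adds the IMC_PlayerCharacter mapping context.
; IA_TakeAndDropObject calls the character's HandleInterract when either its HeldPickup or CarryPoint is valid, leaving the interaction logic to the character.
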(event Input|EnhancedActionEvents|EnhancedInputActionIA_TakeAndDropObject
  (params (ActionValue :type Boolean) (ElapsedSeconds :type Float%20%28double-precision%29) (TriggeredSeconds :type Float%20%28double-precision%29) (InputAction :type Input%20Action%20Object%20Reference :default "/Game/Input/IA_TakeAndDropObject.IA_TakeAndDropObject"))
  ;[0.15 0.15 0.15 0.5] Je vérifie mes is vali pour rantrer dans le handle interract pour gérer interraction objet
  (:Started
    (bind _asbp_character (Utilities|Casting|CastToBP_Character (Pawn|GetControlledPawn)))
    (if (or (Utilities|IsValid (Variables|/Game/Blueprint/Character/BP_Character.BP_Character_C|GetHeldPickup _asbp_character)) (Utilities|IsValid (Variables|/Game/Blueprint/Character/BP_Character.BP_Character_C|GetCarryPoint _asbp_character)))
      (Default|HandleInterract _asbp_character))))

(event EventBeginPlay
  ;[0.15 0.15 0.15 0.5] Posess camera et character
  (bind _returnvalue (Actor|GetActorOfClass "/Game/Blueprint/Character/BP_Character.BP_Character_C"))
  (Pawn|Possess _returnvalue)
  (bind _returnvalue_2 (Actor|GetActorOfClass "/Game/Blueprint/Character/BP_CharacterCamera.BP_CharacterCamera_C"))
  (Game|Player|SetViewTargetwithBlend _returnvalue_2 0.0 "VTBlend_Linear" 0.0 false)
  (Input|AddMappingContext (PlayerController|LocalPlayerSubsystems|GetEnhancedInputLocalPlayerSubsystem) "/Game/Input/IMC_PlayerCharacter.IMC_PlayerCharacter" 0 "(bIgnoreAllPressedKeysUntilRelease=True,bForceImmediately=False,bNotifyUserSettings=False)"))

(fn ConstructionScript)