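; Toy actor that rides a conveyor spline and can be registered as the player character's current pickup.
; On BeginPlay it sets its mesh from DT_Toys by ToyName, finds BP_SplineTapis and starts a looping timer.
; The timer advances it along the spline, destroying it at the end; ClearTimerDeplacement stops movement.
; With ItemTouched set, Collided assigns it to BP_Character's CurrentPickup and collider end overlap clears it.
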(event OnComponentEndOverlap(ColliderNounours)
  (params (OverlappedComponent :type Primitive%20Component%20Object%20Reference) (OtherActor :type Actor%20Object%20Reference) (OtherComp :type Primitive%20Component%20Object%20Reference) (OtherBodyIndex :type Integer))
  ;[0.15 0.15 0.15 0.5] Si je sors de l'ojet je fais oublié qui je suis a bp_character
  (if (Variables|Pickup|GetItemTouched?)
    (bind _asbp_character (Utilities|Casting|CastToBP_Character OtherActor))
    (if (== (Variables|/Game/Blueprint/Character/BP_Character.BP_Character_C|GetCurrentPickup _asbp_character) self)
      (Variables|/Game/Blueprint/Character/BP_Character.BP_Character_C|SetCurrentPickup _asbp_character 0)
      (Variables|Pickup|SetItemTouched? false))))

(event Custom|Move%20Along%20Spline
  (bind _spline (Variables|Cast|GetSpline))
  (bind _spline_2 (Variables|Cast|GetSpline))
  (bind _spline_3 (Variables|/Game/Blueprint/Object/BP_SplineTapis.BP_SplineTapis_C|GetSpline _spline))
  (bind _spline_4 (Variables|/Game/Blueprint/Object/BP_SplineTapis.BP_SplineTapis_C|GetSpline _spline_2))
  ;[0.15 0.15 0.15 0.5] Je vérifie que ma spline existe
  (if (Utilities|IsValid (Variables|Cast|GetSpline))
    ;[0.15 0.15 0.15 0.5] Je règle la distance
    (Variables|Déplacement|SetDistance (+ (Variables|Déplacement|GetDistance) (* (Variables|Déplacement|GetSpeed) (Utilities|Time|GetWorldDeltaSeconds))))
    ;[0.15 0.15 0.15 0.5] Je récupère les points de ma spline pour connaitre le transform et l'orientation
    (if (>= (Variables|Déplacement|GetDistance) (Spline|GetSplineLength _spline_3))
      (Variables|Déplacement|SetDistance (Spline|GetSplineLength _spline_4))
      ;[0.15 0.15 0.15 0.5] Quand il est avant la fin je me déplace ou sinon il se stoppe et se kill
      (Transformation|SetActorLocationAndRotation (Spline|GetLocationatDistanceAlongSpline _spline_4 (Variables|Déplacement|GetDistance) "World") (Spline|GetRotationatDistanceAlongSpline _spline_4 (Variables|Déplacement|GetDistance) "World"))
      (Utilities|Time|ClearandInvalidateTimerbyHandle (Variables|TimeHandler|GetTimer%20Deplacemennt))
      (Actor|DestroyActor)
      (else
        (Transformation|SetActorLocationAndRotation (Spline|GetLocationatDistanceAlongSpline _spline_3 (Variables|Déplacement|GetDistance) "World") (Spline|GetRotationatDistanceAlongSpline _spline_3 (Variables|Déplacement|GetDistance) "World"))))))

(event Custom|Collided
  ;[0.15 0.15 0.15 0.5] Si je rentre dans le collider j'envoie qui je suis a bp_character via current Pickup
  (if (Variables|Pickup|GetItemTouched?)
    (bind _asbp_character (Utilities|Casting|CastToBP_Character (Game|GetPlayerCharacter 0)))
    (Variables|/Game/Blueprint/Character/BP_Character.BP_Character_C|SetCurrentPickup _asbp_character self)))

(event Custom|Clear%20Timer%20Deplacement
  (Utilities|Time|ClearandInvalidateTimerbyHandle (Variables|TimeHandler|GetTimer%20Deplacemennt)))

(event EventBeginPlay
  ;[0.15 0.15 0.15 0.5] Affiche le Static Mesh correspondant au Toy en question
  (bind _returnvalue (Utilities|GetDataTableRow "/Game/Blueprint/Commandes/DT_Toys.DT_Toys" (Variables|Toys|GetToyName))
    (:then
      (Components|StaticMesh|SetStaticMesh (Variables|Default|GetStaticMesh) (.ToyStaticMesh (Utilities|Struct|BreakS_ToysData _returnvalue)))
      ;[0.15 0.15 0.15 0.5] Je récupère ma spline
      (bind _returnvalue_2 (Actor|GetActorOfClass "/Game/Blueprint/Object/BP_SplineTapis.BP_SplineTapis_C"))
      (Variables|Cast|SetSpline _returnvalue_2)
      ;[0.15 0.15 0.15 0.5] Je crée mon event avec son handler
      (bind _returnvalue_3 (Utilities|Time|SetTimerbyEvent (delegate Custom|Move%20Along%20Spline) 0.01 true))
      (Variables|TimeHandler|SetTimer%20Deplacemennt _returnvalue_3))))

(fn ConstructionScript)