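; BP_Nounours is a plush toy object that BP_Character can register as its current pickup.
; Shortly after BeginPlay, a one-shot timer switches on an enum to give the mesh one of several animal materials, such as bear, duck or fox.
; While ItemTouched is true, collider overlaps set the character's CurrentPickup to this toy on entry and clear it on exit if it still points here.
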(event OnComponentEndOverlap(ColliderNounours)
  (params (OverlappedComponent :type Primitive%20Component%20Object%20Reference) (OtherActor :type Actor%20Object%20Reference) (OtherComp :type Primitive%20Component%20Object%20Reference) (OtherBodyIndex :type Integer))
  ;[0.15 0.15 0.15 0.5] Si je sors de l'ojet je fais oublié qui je suis a bp_character
  (if (Variables|Default|GetItemTouched?)
    (bind _asbp_character (Utilities|Casting|CastToBP_Character OtherActor))
    (if (== (Variables|/Game/Blueprint/Character/BP_Character.BP_Character_C|GetCurrentPickup _asbp_character) self)
      (Variables|/Game/Blueprint/Character/BP_Character.BP_Character_C|SetCurrentPickup _asbp_character 0))))

(event OnComponentBeginOverlap(ColliderNounours)
  (params (OverlappedComponent :type Primitive%20Component%20Object%20Reference) (OtherActor :type Actor%20Object%20Reference) (OtherComp :type Primitive%20Component%20Object%20Reference) (OtherBodyIndex :type Integer) (bFromSweep :type Boolean) (SweepResult :type Hit%20Result%20Structure%20%28by%20ref%29))
  ;[0.15 0.15 0.15 0.5] Si je rentre dans le collider j'envoie qui je suis a bp_character via current Pickup
  (if (Variables|Default|GetItemTouched?)
    (bind _asbp_character (Utilities|Casting|CastToBP_Character OtherActor))
    (Variables|/Game/Blueprint/Character/BP_Character.BP_Character_C|SetCurrentPickup _asbp_character self)))

(event Custom|ChoixDuNounours
  ;[0.15 0.15 0.15 0.5] Changement de couleur et de material via un switch un enum et un énumérateur
  (switch Utilities|FlowControl|Switch|SwitchonEnum_Nounours (Variables|Default|GetEnum_Nounours)
    (:NewEnumerator0
      (Rendering|Material|SetMaterial (Variables|Default|GetStaticMesh) 0 "/Game/Materials/Mat_Nounours.Mat_Nounours"))
    (:NewEnumerator1
      (Rendering|Material|SetMaterial (Variables|Default|GetStaticMesh) 0 "/Game/Materials/Mat_Canard.Mat_Canard"))
    (:NewEnumerator2
      (Rendering|Material|SetMaterial (Variables|Default|GetStaticMesh) 0 "/Game/Materials/Mat_Poisson.Mat_Poisson"))
    (:NewEnumerator3
      (Rendering|Material|SetMaterial (Variables|Default|GetStaticMesh) 0 "/Game/Materials/Mat_Lapin.Mat_Lapin"))
    (:NewEnumerator4
      (Rendering|Material|SetMaterial (Variables|Default|GetStaticMesh) 0 "/Game/Materials/Mat_Renard.Mat_Renard"))))

(event EventBeginPlay
  ;[0.15 0.15 0.15 0.5] Changement de couleur et de material via un switch un enum et un énumérateur
  (Utilities|Time|SetTimerbyEvent (delegate Custom|ChoixDuNounours) 0.01))

(fn ConstructionScript)