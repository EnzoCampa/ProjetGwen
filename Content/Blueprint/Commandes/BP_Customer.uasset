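; BP_Customer is a customer that places an order for a toy.
; BeginPlay hides the client mesh and the order widget component.
; StartOrder stores the requested toy, resets remaining patience, then shows the widget and has WB_Order display the toy.
; The file never counts patience down, and its only logic to reveal the mesh is unconnected, so StartOrder leaves the mesh hidden.
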(event EventBeginPlay
  (Rendering|SetVisibility (Variables|Default|GetSM_Client) false true)
  (Rendering|SetVisibility (Variables|Default|GetOrderWidgetComponent) false false))

(fn ConstructionScript)

(fn StartOrder
  (params (SelectedToy :type Name))
  (bind _orderwidgetcomponent (Variables|Default|GetOrderWidgetComponent))
  (Variables|Default|SetRequestedToy SelectedToy)
  (Variables|Default|SetHasOrder? true)
  (Variables|Default|SetRemainingPatience (Variables|Default|GetPatienceTime))
  (Rendering|SetVisibility _orderwidgetcomponent true false)
  (bind _aswb_order (Utilities|Casting|CastToWB_Order (UserInterface|GetUserWidgetObject _orderwidgetcomponent)))
  (Default|DisplayOrder _aswb_order (Variables|Default|GetRequestedToy)))