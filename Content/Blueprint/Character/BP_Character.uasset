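; Player character Blueprint that moves with Enhanced Input, carries pickups and detects BP_Nounours actors.
; Adds its input mapping context on possession or controller change; Move drives camera-relative movement and smoothly turns the actor toward its velocity.
; HandleInterract attaches CurrentPickup to CarryPoint with collision off, or detaches and destroys the held one.
; PickupHolder overlaps swap the character's material and notify the touched Nounours.
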(event OnComponentBeginOverlap(PickupHolder)
  (params (OverlappedComponent :type Primitive%20Component%20Object%20Reference) (OtherActor :type Actor%20Object%20Reference) (OtherComp :type Primitive%20Component%20Object%20Reference) (OtherBodyIndex :type Integer) (bFromSweep :type Boolean) (SweepResult :type Hit%20Result%20Structure%20%28by%20ref%29))
  ;[0.15 0.15 0.15 0.5] J'active ou non le fait de toucher mon nounours
  (bind _asbp_nounours (Utilities|Casting|CastToBP_Nounours OtherActor))
  (Rendering|Material|SetMaterial (Variables|Default|GetCharacter) 0 "/Game/Assets/Materials/Mat_CharacterDetection.Mat_CharacterDetection")
  (Variables|/Game/Blueprint/Object/BP_Nounours.BP_Nounours_C|SetItemTouched? _asbp_nounours true)
  (Default|Collided _asbp_nounours))

(event OnComponentEndOverlap(PickupHolder)
  (params (OverlappedComponent :type Primitive%20Component%20Object%20Reference) (OtherActor :type Actor%20Object%20Reference) (OtherComp :type Primitive%20Component%20Object%20Reference) (OtherBodyIndex :type Integer))
  (Utilities|Casting|CastToBP_Nounours OtherActor)
  (Rendering|Material|SetMaterial (Variables|Default|GetCharacter) 0 "/Game/Assets/Materials/Mat_Character.Mat_Character"))

(event Custom|HandleInterract
  (bind _currentpickup (Variables|Default|GetCurrentPickup))
  ;[0.15 0.15 0.15 0.5] A l'interraction je vérifie si held pickup existe pour récupérer ou poser l'objet
  (if (Utilities|IsValid (Variables|Default|GetHeldPickup))
    ;[0.15 0.15 0.15 0.5] Permet de pose l'onjet attaché
    (Collision|SetCollisionEnabled (Variables|/Game/Blueprint/Object/BP_Nounours.BP_Nounours_C|GetStaticMesh (Variables|Default|GetHeldPickup)) "QueryAndPhysics")
    (Transformation|DetachFromActor (Variables|Default|GetHeldPickup) "KeepWorld" "KeepWorld" "KeepWorld")
    (Actor|DestroyActor (Variables|Default|GetHeldPickup))
    (Variables|Default|SetHeldPickup 0)
    (else
      ;[0.15 0.15 0.15 0.5] Permet de grab l'objet sur mon carry point
      (if (Utilities|IsValid _currentpickup)
        (bind _output_get (Variables|Default|SetHeldPickup _currentpickup))
        (Default|ClearTimerDeplacement _output_get)
        (Collision|SetCollisionEnabled (Variables|/Game/Blueprint/Object/BP_Nounours.BP_Nounours_C|GetStaticMesh _output_get) "NoCollision")
        (Transformation|AttachComponentToComponent _output_get (Variables|Default|GetCarryPoint) "None" "SnapToTarget" "SnapToTarget" "KeepWorld" true)))))

(event Input|EnhancedActionEvents|EnhancedInputActionIA_Move
  (params (ActionValue :type Vector%202D%20Structure) (ElapsedSeconds :type Float%20%28double-precision%29) (TriggeredSeconds :type Float%20%28double-precision%29) (InputAction :type Input%20Action%20Object%20Reference :default "/Game/Input/IA_Move.IA_Move"))
  ;[0.15 0.15 0.15 0.5] Déplacement dans une fonctions move
  (CallFunction|Move (.x ActionValue) (.y ActionValue)))

(event EventControllerChanged
  (params (OldController :type Controller%20Object%20Reference) (NewController :type Controller%20Object%20Reference))
  ;[0.15 0.15 0.15 0.5] Mapping contect
  (bind _asplayer_controller (Utilities|Casting|CastToPlayerController NewController))
  (Input|AddMappingContext (PlayerController|LocalPlayerSubsystems|GetEnhancedInputLocalPlayerSubsystem _asplayer_controller) "/Game/Input/IMC_PlayerCharacter.IMC_PlayerCharacter" 0 "(bIgnoreAllPressedKeysUntilRelease=True,bForceImmediately=False,bNotifyUserSettings=False)"))

(event EventPossessed
  (params (NewController :type Controller%20Object%20Reference))
  ;[0.15 0.15 0.15 0.5] Récupérer l'imc
  (if (Class|Controller|IsPlayerController NewController)
    (bind _asplayer_controller (Utilities|Casting|CastToPlayerController NewController))
    (Input|AddMappingContext (PlayerController|LocalPlayerSubsystems|GetEnhancedInputLocalPlayerSubsystem _asplayer_controller) "/Game/Input/IMC_PlayerCharacter.IMC_PlayerCharacter" 0 "(bIgnoreAllPressedKeysUntilRelease=True,bForceImmediately=False,bNotifyUserSettings=False)")))

(fn ConstructionScript)

(fn Move
  (params (X%20axis :type Float%20%28double-precision%29) (Y%20axis :type Float%20%28double-precision%29))
  (bind _returnvalue (Pawn|GetControlRotation :!class /Script/Engine.Pawn))
  (bind _returnvalue_2 (Transformation|GetVelocity))
  (bind _returnvalue_3 (Math|Vector|MakeVector (.x _returnvalue_2) (.y _returnvalue_2) 0.0))
  ;[0.15 0.15 0.15 0.5] Movement en X et mouvement en Z
  (Pawn|Input|AddMovementInput (Math|Vector|GetRightVector (Math|Rotator|MakeRotator (.roll _returnvalue) 0.0 (.yaw _returnvalue))) X%20axis false)
  (Pawn|Input|AddMovementInput (Math|Vector|GetForwardVector (Math|Rotator|MakeRotator 0.0 0.0 (.yaw (Pawn|GetControlRotation :!class /Script/Engine.Pawn)))) Y%20axis false)
  (if (> (Math|Vector|VectorLength _returnvalue_3) 1.0)
    (Transformation|SetActorRotation (Math|Interpolation|RInterpTo (Transformation|GetActorRotation) (Math|Rotator|MakeRotfromX _returnvalue_3) (Utilities|Time|GetWorldDeltaSeconds) 1e+01))))